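; BP_Hide is an actor Blueprint that fades its dynamic material between partly transparent and opaque.
; Show and Hide set opposing ShouldShow and ShouldHide flags.
; UpdateVisibility steps the Opacity parameter by a given amount, clearing the matching flag at half opacity when hiding or full opacity when showing.
; The event graph and construction script are empty, so nothing here creates the material or calls these functions.
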(event EventBeginPlay)

(event Collision|EventActorBeginOverlap
  (params (OtherActor :type Actor%20Object%20Reference)))

(event EventTick
  (params (DeltaSeconds :type Float%20%28single-precision%29)))

(fn ConstructionScript)

(fn UpdateVisibility
  (params (Amount :type Float%20%28single-precision%29) (ShouldHide :type Boolean))
  (bind _dynamicmaterial (Variables|Default|GetDynamicMaterial))
  (bind _returnvalue (Rendering|Material|GetScalarParameterValue _dynamicmaterial "Opacity" :!class /Script/Engine.MaterialInstanceDynamic))
  (if ShouldHide
    (Rendering|Material|SetScalarParameterValue _dynamicmaterial "Opacity" (- _returnvalue Amount) :!class /Script/Engine.MaterialInstanceDynamic)
    (Variables|Default|SetShouldHide (not (<= (- _returnvalue Amount) 0.5)))
    (else
      (Rendering|Material|SetScalarParameterValue _dynamicmaterial "Opacity" (+ _returnvalue Amount) :!class /Script/Engine.MaterialInstanceDynamic)
      (Variables|Default|SetShouldShow (not (>= (+ _returnvalue Amount) 1.0)))))
  (return))

(fn Show
  (Variables|Default|SetShouldShow true)
  (Variables|Default|SetShouldHide false)
  (return))

(fn Hide
  (Variables|Default|SetShouldHide true)
  (Variables|Default|SetShouldShow false)
  (return))